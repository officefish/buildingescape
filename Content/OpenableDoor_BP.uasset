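; Openable door actor that swings open and closed in response to events from its DoorRotator component.
; The DoorSwing timeline plays on open and reverses on close, applying its OpenAngle as a yaw offset to the rotation saved at BeginPlay.
; An event track on the timeline plays the Doorlock sound at the door's location.
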(event OnOpenEvent(DoorRotator)
  (bind _openangle (Timeline|Door%20Swing Play)
    (:Update
      (Transformation|SetActorRotation (Math|Rotator|CombineRotators (Math|Rotator|MakeRotator 0.0 0.0 _openangle) (Variables|Default|GetInitionalRotation))))
    (:Sound%20Timing
      (Audio|PlaySoundatLocation "/Game/Audio/door-lock.door-lock" (Transformation|GetActorLocation)))))

(event OnCloseEvent(DoorRotator)
  (bind _openangle (Timeline|Door%20Swing Reverse)
    (:Update
      (Transformation|SetActorRotation (Math|Rotator|CombineRotators (Math|Rotator|MakeRotator 0.0 0.0 _openangle) (Variables|Default|GetInitionalRotation))))
    (:Sound%20Timing
      (Audio|PlaySoundatLocation "/Game/Audio/door-lock.door-lock" (Transformation|GetActorLocation)))))

(event EventBeginPlay
  (Variables|Default|SetInitionalRotation (Transformation|GetActorRotation)))

(fn ConstructionScript)